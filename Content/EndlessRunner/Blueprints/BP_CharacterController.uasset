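; Player controller for an endless runner that owns the HUD, coin score, rising game speed and death handling.
; BeginPlay creates the HUD and starts a looping timer that nudges GameSpeed up and applies it as global time dilation, accelerating the whole game.
; CollectCoin increments the score and pushes it to the HUD.
; PlayerDeath pauses the game, shows the death screen and reveals the mouse cursor.
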(event Custom|Event%20CollectCoin
  (bind _result (Math|Integer|IncrementInt (Variables|Default|GetScore))
    (:%20%20
      (bind _output_get (Variables|Default|SetScore _result))
      (Default|SetScore (Variables|Default|GetHUD) _output_get))))

(event Custom|Event%20PlayerDeath
  (Game|SetGamePaused true)
  (Default|ShowDeathScreen (Variables|Default|GetHUD))
  (Variables|Default|SetbShowMouseCursor true))

(event EventBeginPlay
  (bind _returnvalue (UserInterface|CreateWidget "/Game/EndlessRunner/Blueprints/BP_HUD.BP_HUD_C"))
  (bind _output_get (Variables|Default|SetHUD _returnvalue))
  (UserInterface|Viewport|AddtoViewport _output_get 0)
  (Default|SetScore _output_get)
  (bind _returnvalue_2 (Utilities|Time|SetTimerbyFunctionName 0 "IncreaseGlobalTime" 1.0 true))
  (Variables|Default|SetGlobalTimeTimer _returnvalue_2)
  (Variables|Default|SetbShowMouseCursor false))

(fn ConstructionScript)

(fn IncreaseGlobalTime
  (if (not (Game|IsGamePaused))
    (bind _output_get (Variables|Default|SetGameSpeed (+ (Variables|Default|GetGameSpeed) 0.01)))
    (Utilities|Time|SetGlobalTimeDilation _output_get)))