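; Shared helper library for the endless runner, covering movement and lane-grid placement.
; MoveBackwards shifts a target actor along the X axis by Speed scaled with delta time, without sweeping.
; Column and line helpers convert indices into evenly spaced offsets, and GetRandomColumn picks one of three columns centered on zero.
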(fn MoveBackwards
  (params (Target :type Actor%20Object%20Reference) (DeltaSeconds :type Float%20%28double-precision%29))
  (Transformation|SetActorLocation Target (+ (Transformation|GetActorLocation Target) (* (Math|Vector|MakeVector (LocalVariables|GetSpeed) 0.0 0.0) DeltaSeconds)) false false))

(fn GetColumnPosition
  (params (Column :type Integer))
  (return (* Column 1.6e+02)))

(fn GetLinePosition
  (params (Index :type Integer))
  (return (* Index 1e+02)))

(fn GetRandomColumn
  (return (Math|Random|RandomIntegerinRange -1 1)))