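; Endless runner obstacle that moves backwards every tick and damages the player character on contact.
; An actor overlap casts the other actor to BP_Character and applies one point of damage.
; SetPosition places it at line 0 in a given column, keeping its height, and prints a debug string.
; The movement and grid position helpers it calls are defined outside this graph.
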(event EventTick
  (params (DeltaSeconds :type Float%20%28single-precision%29))
  (CallFunction|MoveBackwards self DeltaSeconds))

(event Collision|EventActorBeginOverlap
  (params (OtherActor :type Actor%20Object%20Reference))
  (bind _asbp_character (Utilities|Casting|CastToBP_Character OtherActor))
  (Game|Damage|ApplyDamage _asbp_character 1.0 0 0))

(fn ConstructionScript)

(fn SetPosition
  (params (Column :type Integer))
  (Transformation|SetActorLocation (Math|Vector|MakeVector (CallFunction|GetLinePosition) (CallFunction|GetColumnPosition Column) (.z (Transformation|GetActorLocation))) false false)
  (Development|PrintString "SET POS"))