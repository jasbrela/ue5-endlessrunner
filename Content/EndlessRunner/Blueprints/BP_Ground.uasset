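; BP_Ground is an endless-runner ground segment that moves backwards every tick and recycles its linked segment.
; When the player overlaps it with CanTrigger set, it repositions NextGround a fixed X offset ahead of itself, debounced by a DoOnce and short delay.
; A repositioned segment enables its trigger, picks a random column and repositions valid BP_Collectable actors, cached at BeginPlay, there up to the MaxCoins index.
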(event EventBeginPlay
  (bind _outactors (Actor|GetAllActorsOfClass "/Game/EndlessRunner/Blueprints/BP_Collectable.BP_Collectable_C"))
  (Variables|Default|SetCollectables _outactors))

(event EventTick
  (params (DeltaSeconds :type Float%20%28single-precision%29))
  (CallFunction|MoveBackwards self DeltaSeconds))

(event Collision|EventActorBeginOverlap
  (params (OtherActor :type Actor%20Object%20Reference))
  (if (== OtherActor (Game|Player|GetPlayerPawn 0))
    (if (Variables|Default|GetCan%20Trigger)
      (Utilities|FlowControl|DoOnce false :!label _label
        (:Completed
          (CallFunction|SetPosition (Variables|Default|GetNext%20Ground) (Transformation|GetActorLocation))
          (Utilities|FlowControl|Delay 0.2)
          (goto _label Reset))))
    (else
      (Development|PrintString (Utilities|GetDisplayName OtherActor)))))

(fn ConstructionScript)

(fn SetPosition
  (params (Position :type Vector))
  (Transformation|SetActorLocation (Math|Vector|MakeVector (+ (.x Position) 2.2e+03) 0.0 0.0) false false)
  (Variables|Default|SetCan%20Trigger true)
  (if true
    (bind _output_get (Variables|Default|SetColumn (Math|Random|RandomIntegerinRange -1 1)))
    (Utilities|UpdateValidCollectables)
    (for (_array_element _array_index) (Variables|Default|GetValid%20Collectables)
      (if (>= (Variables|Default|GetMaxCoins) _array_index)
        (Default|SetPosition _array_element _array_index _output_get)))))